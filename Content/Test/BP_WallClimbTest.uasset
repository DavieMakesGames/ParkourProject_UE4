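; BP_WallClimbTest is a functional test that checks whether a character can get to a trigger, named for wall climbing.
; On start it binds the trigger's overlap event, then sends the character a jump message after a short delay.
; Tick constantly pushes forward movement input along the character's facing.
; The test succeeds when that character overlaps the trigger; the graph defines no failure path of its own.
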(event Custom|OnActorBeginOverlap_Event_0
  (params (OverlappedActor :type Actor%20Object%20Reference) (OtherActor :type Actor%20Object%20Reference))
  (if (== OtherActor (Variables|Default|GetCharacter))
    (Class|FunctionalTest|FinishTest "Succeeded")))

(event Custom|Bind%20Trigger
  (EventDispatchers|AssignOnActorBeginOverlap (Variables|Default|GetTrigger) (delegate Custom|OnActorBeginOverlap_Event_0)))

(event EventPrepareTest)

(event EventStartTest
  (CallFunction|BindTrigger)
  (Utilities|FlowControl|Delay 1.0)
  (Class|MobileInterface|JumpEvent(Message) (Variables|Default|GetCharacter)))

(event EventTick
  (params (DeltaSeconds :type Float%20%28single-precision%29))
  (bind _character (Variables|Default|GetCharacter))
  (Pawn|Input|AddMovementInput _character (Transformation|GetActorForwardVector _character) 1.0 false))

(fn ConstructionScript)